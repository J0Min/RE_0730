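; BP_Enermy is an AI-controlled melee enemy that targets the player, attacks, reacts to hits and dies.
; TempDetector overlap hands the player to AIC_Enermy as target, and StartAttack sets a timer for a right-arm sphere trace that damages Player-tagged actors.
; Damage spawns blood and reduces health through BPCStatSystem, then triggers either knockback with a random hit montage or death and delayed destruction.
; Hit and death states are mirrored to the Blackboard.
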(event OnComponentBeginOverlap(TempDetector)
  (params (OverlappedComponent :type Primitive%20Component%20Object%20Reference) (OtherActor :type Actor%20Object%20Reference) (OtherComp :type Primitive%20Component%20Object%20Reference) (OtherBodyIndex :type Integer) (bFromSweep :type Boolean) (SweepResult :type Hit%20Result%20Structure%20%28by%20ref%29))
  (bind _asbp_player_character_fixed_vivian (Utilities|Casting|CastToBP_PlayerCharacter_FixedVivian OtherActor))
  (bind _asaic_enermy (Utilities|Casting|CastToAIC_Enermy (AI|GetAIController self)))
  (Default|SetTarget _asaic_enermy _asbp_player_character_fixed_vivian))

(event Custom|Attack
  (bind (_outhit _returnvalue) (Collision|SphereTraceByChannel (Transformation|GetWorldLocation (Variables|Default|GetRightArmStart)) (Transformation|GetWorldLocation (Variables|Default|GetRightArmEnd)) 3e+01 "TraceTypeQuery1" false 0 "ForDuration"))
  (if _returnvalue
    (if (Actor|ActorHasTag (.HitActor (Collision|BreakHitResult _outhit)) "Player")
      (Game|Damage|ApplyDamage (.HitActor (Collision|BreakHitResult _outhit)) 2e+01 0 self))))

(event Custom|StartAttack
  (bind _returnvalue (Utilities|Time|SetTimerbyEvent (delegate Custom|Attack) 0.01))
  (Variables|Default|SetAttackTimerHandler _returnvalue))

(event Custom|StopAttack
  (Utilities|Time|ClearandInvalidateTimerbyHandle (Variables|Default|GetAttackTimerHandler)))

(event EventBeginPlay
  (bind _asabp_enermy (Utilities|Casting|CastToABP_Enermy (Components|SkeletalMesh|GetAnimInstance (Variables|Character|GetMesh))))
  (Variables|Default|SetAnimationBP _asabp_enermy))

(event Game|Damage|EventAnyDamage
  (params (Damage :type Float%20%28single-precision%29) (DamageType :type Damage%20Type%20Object%20Reference) (InstigatedBy :type Controller%20Object%20Reference) (DamageCauser :type Actor%20Object%20Reference))
  (Utilities|FlowControl|Sequence
    (:then_0
      (bind _output_get (Variables|Default|SetIsHit true))
      (AI|Components|Blackboard|SetValueasBool (AI|GetBlackboard 0) (Variables|Default|GetIsHitBlackboardKey) _output_get))
    (:then_1
      (Variables|Default|SetDamage%20Causer DamageCauser)
      (Niagara|SpawnSystematLocation "/Game/Hobby_introduction/VFX/HitImpact/NS_HitBlood.NS_HitBlood" (Variables|Default|GetHitLocation))
      (bind _isdeath (Default|DecreaseHealth (Variables|Default|GetBPC_StatSystem) Damage))
      (bind _output_get_2 (Variables|Default|SetIs%20Death _isdeath))
      (if _output_get_2
        (AI|Components|Blackboard|SetValueasBool (AI|GetBlackboard 0) (Variables|Default|GetIsDeadBlackboardKey) _output_get_2)
        (Animation|PlayAnimMontage "/Game/Hobby_introduction/Animations/Montages/Death_Montage.Death_Montage" 1.0 "None")
        (Collision|SetCollisionEnabled (Variables|Collision|GetCapsuleComponent) "NoCollision")
        (Utilities|FlowControl|Delay 5.0)
        (Actor|DestroyActor)
        (else
          (CallFunction|SetBackEnermyLocation)
          (bind _delaytime (CallFunction|PlayHitAnimaion (Variables|Default|GetHitAnimations)))
          (Utilities|FlowControl|Delay _delaytime) ; 애니메이션이 종료될때까지 지연(Delay) 된다.
          (bind _output_get_3 (Variables|Default|SetIsHit false))
          (AI|Components|Blackboard|SetValueasBool (AI|GetBlackboard 0) (Variables|Default|GetIsHitBlackboardKey) _output_get_3))))))

(fn ConstructionScript)

(fn PlayHitAnimaion
  (params (TargetArray :type Array%20of%20Anim%20Montage%20Object%20References))
  (bind _returnvalue (Animation|PlayAnimMontage (Utilities|Array|Get(acopy) TargetArray (Math|Random|RandomIntegerinRange 0 (- (Utilities|Array|Length TargetArray) 1))) 1.0 "None"))
  (return _returnvalue))

(fn SetBackEnermyLocation
  (Transformation|SetActorLocation (+ (* (Transformation|GetActorForwardVector (Variables|Default|GetDamage%20Causer)) 20) (Transformation|GetActorLocation)) false false) ; 맞으면 플레이어가 바라보는 방향으로 20만큼 이동\n즉, 맞으면 뒤로 밀려나는 느낌
)