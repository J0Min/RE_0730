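; Actor component that manages quick slots, filled by dragging items from the inventory.
; On BeginPlay it sizes the QuickSlots array to QuickSlotSize.
; The MouseDropToQuickSlot event calls AddToQuickSlot, which copies the chosen entry from the passed inventory component's Slots into the target index and broadcasts OnQuickSlotUpdate.
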(event Custom|MouseDropToQuickSlot
  (params (TargetQuickSlotInex :type Integer) (BPC_InventorySystem :type BPC%20Inventory%20System%20Object%20Reference) (InventoryItemIndex :type Integer))
  (CallFunction|AddtoQuickSlot TargetQuickSlotInex BPC_InventorySystem InventoryItemIndex))

(event EventBeginPlay
  (Utilities|Array|Resize (Variables|Default|GetQuickSlots) (Variables|Default|GetQuickSlotSize)))

(fn AddtoQuickSlot
  (params (TargetQuickSlotInex :type Integer) (BPC_InventorySystem :type BPC%20Inventory%20System%20Object%20Reference) (InventoryItemIndex :type Integer))
  (Utilities|Array|SetArrayElem (Variables|Default|GetQuickSlots) TargetQuickSlotInex (Utilities|Array|Get(acopy) (Variables|/Game/Hobby_introduction/Inventory/Inventory/BPC_InventorySystem.BPC_InventorySystem_C|GetSlots BPC_InventorySystem) InventoryItemIndex))
  (Default|CallOnQuickSlotUpdate))