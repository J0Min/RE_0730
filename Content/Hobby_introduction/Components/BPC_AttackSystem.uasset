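; Player attack component handling a four-hit unarmed punch combo, plus rifle firing and aiming when armed.
; Montage notifies advance the combo, which resets by timer or hit interruption; StartAttackTrace schedules a hand sphere trace that applies damage.
; Rifle fire plays effects, then line-traces from camera and muzzle to damage BP_Enermy.
; Aiming toggles zoom, crosshair and orient-to-movement.
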(event Custom|ResetCount
  (Variables|Default|SetComboCount 0))

(event Custom|AttackTrace
  (bind _playercharacter (Variables|Default|GetPlayerCharacter))
  (bind _playercharacter_2 (Variables|Default|GetPlayerCharacter))
  (bind _righthand (Variables|/Game/Hobby_introduction/Player/BP_PlayerCharacter_FixedVivian.BP_PlayerCharacter_FixedVivian_C|GetRightHand _playercharacter_2))
  (bind _lefthand (Variables|/Game/Hobby_introduction/Player/BP_PlayerCharacter_FixedVivian.BP_PlayerCharacter_FixedVivian_C|GetLeftHand _playercharacter))
  (bind (_start _end) (CallFunction|GetHandLocation _lefthand))
  (bind (_start_2 _end_2) (CallFunction|GetHandLocation _righthand))
  (switch int (Variables|Default|GetComboCount)
    (:0
      (CallFunction|AttackSphereTrace (Variables|Default|GetBase%20Damage) (Variables|Default|GetPlayerCharacter) _start _end :!label _label))
    (:1
      (CallFunction|AttackSphereTrace (Variables|Default|GetBase%20Damage) (Variables|Default|GetPlayerCharacter) _start_2 _end_2 :!label _label_2))
    (:2
      (goto _label))
    (:3
      (goto _label_2))))

(event Custom|StartAttackTrace
  (bind _returnvalue (Utilities|Time|SetTimerbyEvent (delegate Custom|AttackTrace) 0.01))
  (Variables|Default|SetAttackTimerHandler _returnvalue))

(event Custom|ResetByHIt
  (if (Variables|/Game/Hobby_introduction/Player/BP_PlayerCharacter_FixedVivian.BP_PlayerCharacter_FixedVivian_C|GetIsHiting (Variables|Default|GetPlayerCharacter))
    (Variables|Default|SetIsAttacking false)
    (Variables|Default|SetComboCount 0)))

(event Custom|StopAttackTrace
  (Utilities|Time|ClearandInvalidateTimerbyHandle (Variables|Default|GetAttackTimerHandler)))

(event Custom|RifleFire
  (bind _playercharacter (Variables|Default|GetPlayerCharacter))
  (bind _playercharacter_2 (Variables|Default|GetPlayerCharacter))
  (bind _camera (Variables|/Game/Hobby_introduction/Player/BP_PlayerCharacter_FixedVivian.BP_PlayerCharacter_FixedVivian_C|GetCamera _playercharacter))
  (bind _currentweapon (Variables|/Game/Hobby_introduction/Player/BP_PlayerCharacter_FixedVivian.BP_PlayerCharacter_FixedVivian_C|GetCurrentWeapon _playercharacter_2))
  (bind _returnvalue (Transformation|GetWorldLocation _camera))
  (bind _returnvalue_2 (Math|Vector|GetForwardVector _camera))
  (bind _weapon (Variables|/Game/Hobby_introduction/Items/Weapons/BP_WeaponMaster.BP_WeaponMaster_C|GetWeapon _currentweapon))
  (bind _returnvalue_3 (Transformation|GetSocketLocation _weapon "Muzzle"))
  (bind _returnvalue_4 (* _returnvalue_2 2e+04))
  (Animation|Montage|PlayMontage (Variables|/Script/Engine.Character|GetMesh (Variables|Default|GetPlayerCharacter)) "/Game/Hobby_introduction/Animations/FireAnimation/MM_Rifle_Fire_Montage.MM_Rifle_Fire_Montage"
    (:then
      (CallFunction|PlayMuzzleFlash)
      (bind (_outhit _returnvalue_5) (Collision|LineTraceByChannel _returnvalue (+ _returnvalue _returnvalue_4) "TraceTypeQuery1" false 0 "None")) ; 카메라 기준 조준
      (if _returnvalue_5
        (bind (_outhit_2 _returnvalue_6) (Collision|LineTraceByChannel _returnvalue_3 (* (Math|Vector|Normalize (- (.ImpactPoint (Collision|BreakHitResult _outhit)) _returnvalue_3)) 2e+04) "TraceTypeQuery1" false 0 "None"))
        (if _returnvalue_6
          (bind _asbp_enermy (Utilities|Casting|CastToBP_Enermy (.HitActor (Collision|BreakHitResult _outhit_2))))
          (Variables|/Game/Hobby_introduction/Enermy/BP_Enermy.BP_Enermy_C|SetHitLocation _asbp_enermy (.ImpactPoint (Collision|BreakHitResult _outhit_2)))
          (Game|Damage|ApplyDamage (.HitActor (Collision|BreakHitResult _outhit_2)) 33.0 0 (Variables|Default|GetPlayerCharacter)))
        (else
          (Collision|LineTraceByChannel _returnvalue_3 (+ _returnvalue_3 _returnvalue_4) "TraceTypeQuery1" false 0 "None"))))))

(event Input|EnhancedActionEvents|EnhancedInputActionIA_Attack
  (params (ActionValue :type Boolean) (ElapsedSeconds :type Float%20%28double-precision%29) (TriggeredSeconds :type Float%20%28double-precision%29) (InputAction :type Input%20Action%20Object%20Reference :default "/Game/Hobby_introduction/Player/Inputs/IA_Attack.IA_Attack"))
  (bind _charactermesh (Variables|Default|GetCharacterMesh))
  (bind _charactermesh_2 (Variables|Default|GetCharacterMesh))
  (:Started
    (if (Variables|/Game/Hobby_introduction/Player/BP_PlayerCharacter_FixedVivian.BP_PlayerCharacter_FixedVivian_C|GetIsArmedRifle (Variables|Default|GetPlayerCharacter))
      (CallFunction|RifleFire)
      (elif (and (not (Variables|Default|GetIsAttacking)) (not (Variables|/Game/Hobby_introduction/Player/BP_PlayerCharacter_FixedVivian.BP_PlayerCharacter_FixedVivian_C|GetIsHiting (Variables|Default|GetPlayerCharacter)))) ; 공격 중이 아닐때 만 TRUE
        (Variables|Default|SetIsAttacking true)
        (switch int (Variables|Default|GetComboCount) ; Swith case문
          (:0
            (Animation|Montage|PlayMontage _charactermesh_2 "/Game/Hobby_introduction/Animations/Montages/Attack1_Jab_Montage.Attack1_Jab_Montage" ; 캐릭터의 애니메이션 조절
              (:then
                (Utilities|Time|SetTimerbyEvent (delegate Custom|ResetCount) 1.0 :!label _label))
              (:OnInterrupted
                (CallFunction|ResetbyHIt :!label _label_2))
              (:OnNotifyBegin
                (Variables|Default|SetIsAttacking false)
                (Variables|Default|SetComboCount 1))))
          (:1
            (Animation|Montage|PlayMontage _charactermesh_2 "/Game/Hobby_introduction/Animations/Montages/Attack2_Straight_Montage.Attack2_Straight_Montage"
              (:then
                (goto _label))
              (:OnInterrupted
                (goto _label_2))
              (:OnNotifyBegin
                (Variables|Default|SetIsAttacking false)
                (Variables|Default|SetComboCount 2))))
          (:2
            (Animation|Montage|PlayMontage _charactermesh "/Game/Hobby_introduction/Animations/Montages/Attack3_Hook_Montage.Attack3_Hook_Montage"
              (:then
                (goto _label))
              (:OnInterrupted
                (CallFunction|ResetbyHIt :!label _label_3))
              (:OnNotifyBegin
                (Variables|Default|SetIsAttacking false)
                (Variables|Default|SetComboCount 3))))
          (:3
            (Animation|Montage|PlayMontage _charactermesh "/Game/Hobby_introduction/Animations/Montages/Attack4_Hook_Montage.Attack4_Hook_Montage"
              (:then
                (goto _label))
              (:OnInterrupted
                (goto _label_3))
              (:OnNotifyBegin
                (Variables|Default|SetIsAttacking false)
                (Variables|Default|SetComboCount 0)))))))))

(event Input|EnhancedActionEvents|EnhancedInputActionIA_Aiming
  (params (ActionValue :type Boolean) (ElapsedSeconds :type Float%20%28double-precision%29) (TriggeredSeconds :type Float%20%28double-precision%29) (InputAction :type Input%20Action%20Object%20Reference :default "/Game/Hobby_introduction/Player/Inputs/IA_Aiming.IA_Aiming"))
  (bind _playercharacter (Variables|Default|GetPlayerCharacter))
  (bind _playercharacter_2 (Variables|Default|GetPlayerCharacter))
  (bind _playercontroller (Variables|/Game/Hobby_introduction/Player/BP_PlayerCharacter_FixedVivian.BP_PlayerCharacter_FixedVivian_C|GetPlayerController _playercharacter_2))
  (bind _playerhud (Variables|/Game/Hobby_introduction/Player/BP_PlayerController.BP_PlayerController_C|GetPlayerHUD _playercontroller))
  (bind _crosshair (Variables|/Game/Hobby_introduction/UI/WB_HUD.WB_HUD_C|GetCrosshair _playerhud))
  (:Triggered
    (if (Variables|/Game/Hobby_introduction/Player/BP_PlayerCharacter_FixedVivian.BP_PlayerCharacter_FixedVivian_C|GetIsArmedRifle (Variables|Default|GetPlayerCharacter))
      (Variables|Default|SetIsAming true)
      (Variables|/Script/Engine.CharacterMovementComponent|SetbOrientRotationToMovement (Variables|/Script/Engine.Character|GetCharacterMovement (Variables|Default|GetPlayerCharacter)) false)
      (Default|ZoominbyAiming _playercharacter)
      (Widget|SetVisibility _crosshair "Visible")))
  (:Canceled
    (if (Variables|/Game/Hobby_introduction/Player/BP_PlayerCharacter_FixedVivian.BP_PlayerCharacter_FixedVivian_C|GetIsArmedRifle (Variables|Default|GetPlayerCharacter)) :!label _label
      (Variables|Default|SetIsAming false)
      (Variables|/Script/Engine.CharacterMovementComponent|SetbOrientRotationToMovement (Variables|/Script/Engine.Character|GetCharacterMovement (Variables|Default|GetPlayerCharacter)) true)
      (Default|ZoomOutbyAimingEnd _playercharacter)
      (Widget|SetVisibility _crosshair "Hidden")))
  (:Completed
    (goto _label)))

(event EventBeginPlay
  (bind _asbp_player_character_fixed_vivian (Utilities|Casting|CastToBP_PlayerCharacter_FixedVivian (Components|GetOwner)))
  (bind _output_get (Variables|Default|SetPlayerCharacter _asbp_player_character_fixed_vivian))
  (Variables|Default|SetCharacterMesh (Variables|/Script/Engine.Character|GetMesh _output_get)))

(fn GetHandLocation
  (params (Hand :type Scene%20Component%20Object%20Reference))
  (return (Transformation|GetWorldLocation Hand) (Math|Transform|TransformLocation (Transformation|GetWorldTransform Hand) (+ (Variables|/Script/Engine.SceneComponent|GetRelativeLocation Hand) (Math|Vector|MakeVector 2e+01 0.0 0.0)))) ; 퓨어 함수로 변경 > 함수의 입력출력 단계를 안만듦.
)

(fn AttackSphereTrace
  (params (BaseDamage :type Float%20%28single-precision%29) (DamageCauser :type Actor%20Object%20Reference) (Start :type Vector) (End :type Vector))
  (bind (_outhit _returnvalue) (Collision|SphereTraceByChannel Start End 1e+01 "TraceTypeQuery1" false 0 "ForDuration" true "(R=1.000000,G=0.000000,B=0.000000,A=1.000000)" "(R=0.000000,G=1.000000,B=0.000000,A=1.000000)" 7.0))
  (if _returnvalue
    (Game|Damage|ApplyDamage (.HitActor (Collision|BreakHitResult _outhit)) BaseDamage 0 DamageCauser)))

(fn PlayMuzzleFlash
  (bind _playercharacter (Variables|Default|GetPlayerCharacter))
  (bind _currentweapon (Variables|/Game/Hobby_introduction/Player/BP_PlayerCharacter_FixedVivian.BP_PlayerCharacter_FixedVivian_C|GetCurrentWeapon _playercharacter))
  (bind _weapon (Variables|/Game/Hobby_introduction/Items/Weapons/BP_WeaponMaster.BP_WeaponMaster_C|GetWeapon _currentweapon))
  (bind _returnvalue (Transformation|GetSocketLocation _weapon "Muzzle"))
  (Effects|SpawnEmitteratLocation "/Game/MilitaryWeapDark/FX/P_AssaultRifle_MuzzleFlash.P_AssaultRifle_MuzzleFlash" _returnvalue)
  (Audio|PlaySoundatLocation "/Game/MilitaryWeapDark/Sound/Rifle/RifleB_Fire_Cue.RifleB_Fire_Cue" _returnvalue "0, 0, 0" 1.0 1.0 0.0 0 0 0 0))