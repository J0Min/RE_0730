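; Health stat component for the player and enemies that tracks current health and reports death.
; On BeginPlay it finds the first WB_HUD widget and, only if one exists, fills health to max and caches the widget.
; Increase and decrease functions take the HUD as a parameter and update its health bar before clamping the value.
; DecreaseHealth skips the bar when no HUD is passed, as for enemies, and returns IsDeath.
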(event EventBeginPlay
  (bind _foundwidgets (Widget|GetAllWidgetsOfClass "/Game/Hobby_introduction/UI/WB_HUD.WB_HUD_C" true))
  (Utilities|IsValid (Utilities|Array|Get(acopy) _foundwidgets)
    (:Is%20Valid
      (CallFunction|IntializeStat (Utilities|Array|Get(acopy) _foundwidgets))
      (Variables|Default|SetPlayerHUD (Utilities|Array|Get(acopy) _foundwidgets)))))

(event EventTick
  (params (DeltaSeconds :type Float%20%28single-precision%29)))

(fn IncreaseHealth
  (params (HealthPoint :type Float%20%28double-precision%29) (PlayerHUD :type WB%20HUD%20Object%20Reference))
  (bind _output_get (Variables|Default|SetCurrentHealth (+ HealthPoint (Variables|Default|GetCurrentHealth))))
  (Default|SetHealthBarPercent PlayerHUD _output_get (Variables|Default|GetMaxHealth))
  (if (>= (Variables|Default|GetCurrentHealth) (Variables|Default|GetMaxHealth))
    (Variables|Default|SetCurrentHealth (Variables|Default|GetMaxHealth))))

(fn DecreaseHealth
  (params (DamagePoint :type Float%20%28double-precision%29) (PlayerHUD :type WB%20HUD%20Object%20Reference))
  (Variables|Default|SetCurrentHealth (- (Variables|Default|GetCurrentHealth) DamagePoint))
  (bind _playerhud (LocalVariables|GetPlayerHUD) ; 플레이어에게는 있지만 적에게는 없어서 이부분이 오류 발생
    (:then
      (Default|SetHealthBarPercent _playerhud (Variables|Default|GetCurrentHealth) (Variables|Default|GetMaxHealth)))
    (:else
      _))
  (if (<= (Variables|Default|GetCurrentHealth) 0.0)
    (Variables|Default|SetCurrentHealth 0.0)
    (bind _output_get (Variables|Default|SetIsDeath true))
    (return _output_get)
    (else
      (bind _output_get_2 (Variables|Default|SetIsDeath false))
      (return _output_get_2))))

(fn IntializeStat
  (params (PlayerHUD :type WB%20HUD%20Object%20Reference))
  (bind _output_get (Variables|Default|SetCurrentHealth (Variables|Default|GetMaxHealth)))
  (Default|SetHealthBarPercent PlayerHUD _output_get (Variables|Default|GetMaxHealth)))