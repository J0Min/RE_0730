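; BP_Enermy is an enemy character that detects the player, takes damage and dies.
; An overlap on TempDetector passes the Vivian player character to its AI controller as the target.
; AnyDamage reduces health through the stat component; non-lethal hits play a random hit montage, a sound and nudge it along the attacker's forward vector.
; Death notifies the animation Blueprint, disables capsule collision and destroys the actor after a delay.
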(event OnComponentBeginOverlap(TempDetector)
  (params (OverlappedComponent :type Primitive%20Component%20Object%20Reference) (OtherActor :type Actor%20Object%20Reference) (OtherComp :type Primitive%20Component%20Object%20Reference) (OtherBodyIndex :type Integer) (bFromSweep :type Boolean) (SweepResult :type Hit%20Result%20Structure%20%28by%20ref%29))
  (bind _asbp_player_character_fixed_vivian (Utilities|Casting|CastToBP_PlayerCharacter_FixedVivian OtherActor))
  (bind _asaic_enermy (Utilities|Casting|CastToAIC_Enermy (AI|GetAIController self)))
  (Default|SetTarget _asaic_enermy _asbp_player_character_fixed_vivian))

(event EventBeginPlay
  (bind _asabp_enermy (Utilities|Casting|CastToABP_Enermy (Components|SkeletalMesh|GetAnimInstance (Variables|Character|GetMesh))))
  (Variables|Default|SetAnimationBP _asabp_enermy))

(event Game|Damage|EventAnyDamage
  (params (Damage :type Float%20%28single-precision%29) (DamageType :type Damage%20Type%20Object%20Reference) (InstigatedBy :type Controller%20Object%20Reference) (DamageCauser :type Actor%20Object%20Reference))
  (Variables|Default|SetDamage%20Causer DamageCauser)
  (bind _isdeath (Default|DecreaseHealth (Variables|Default|GetBPC_StatSystem) Damage))
  (bind _output_get (Variables|Default|SetIs%20Death _isdeath))
  (if _output_get
    (Default|SetEnermyIsDead (Variables|Default|GetAnimationBP))
    (Collision|SetCollisionEnabled (Variables|Collision|GetCapsuleComponent) "NoCollision")
    (Utilities|FlowControl|Delay 5.0)
    (Actor|DestroyActor)
    (else
      (CallFunction|PlayHitAnimaion (Variables|Default|GetHitAnimations))
      (CallFunction|SetBackEnermyLocation)
      (Audio|PlaySound2D "/Game/StarterContent/Audio/Collapse01.Collapse01" 1.0 1.0 2.0 0 0))))

(fn ConstructionScript)

(fn PlayHitAnimaion
  (params (TargetArray :type Array%20of%20Anim%20Montage%20Object%20References))
  (Animation|PlayAnimMontage (Utilities|Array|Get(acopy) TargetArray (Math|Random|RandomIntegerinRange 0 (- (Utilities|Array|Length TargetArray) 1))) 1.0 "None"))

(fn SetBackEnermyLocation
  (Transformation|SetActorLocation (+ (* (Transformation|GetActorForwardVector (Variables|Default|GetDamage%20Causer)) 20) (Transformation|GetActorLocation)) false false) ; 맞으면 플레이어가 바라보는 방향으로 20만큼 이동\n즉, 맞으면 뒤로 밀려나는 느낌
)