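; BPC_StatSystem is a component that tracks health and reports death when it runs out.
; On BeginPlay it finds the first top-level WB_HUD widget and, if valid, initializes current health to maximum.
; IncreaseHealth and DecreaseHealth update the passed HUD's health bar before clamping the value at its respective limit.
; DecreaseHealth also sets and returns the IsDeath flag.
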(event EventBeginPlay
  (bind _foundwidgets (Widget|GetAllWidgetsOfClass "/Game/NEW/UI/WB_HUD.WB_HUD_C" true))
  (Utilities|IsValid (Utilities|Array|Get(acopy) _foundwidgets)
    (:Is%20Valid
      (CallFunction|IntializeStat (Utilities|Array|Get(acopy) _foundwidgets)))))

(event EventTick
  (params (DeltaSeconds :type Float%20%28single-precision%29)))

(fn IncreaseHealth
  (params (HealthPoint :type Float%20%28double-precision%29) (PlayerHUD :type WB%20HUD%20Object%20Reference))
  (bind _output_get (Variables|Default|SetCurrentHealth (+ HealthPoint (Variables|Default|GetCurrentHealth))))
  (Default|SetHealthBarPercent PlayerHUD _output_get (Variables|Default|GetMaxHealth))
  (if (>= (Variables|Default|GetCurrentHealth) (Variables|Default|GetMaxHealth))
    (Variables|Default|SetCurrentHealth (Variables|Default|GetMaxHealth))))

(fn DecreaseHealth
  (params (DamagePoint :type Float%20%28double-precision%29) (PlayerHUD :type WB%20HUD%20Object%20Reference))
  (bind _output_get (Variables|Default|SetCurrentHealth (- (Variables|Default|GetCurrentHealth) DamagePoint)))
  (Default|SetHealthBarPercent PlayerHUD _output_get (Variables|Default|GetMaxHealth))
  (if (<= (Variables|Default|GetCurrentHealth) 0.0)
    (Variables|Default|SetCurrentHealth 0.0)
    (bind _output_get_2 (Variables|Default|SetIsDeath true))
    (return _output_get_2)
    (else
      (bind _output_get_3 (Variables|Default|SetIsDeath false))
      (return _output_get_3))))

(fn IntializeStat
  (params (PlayerHUD :type WB%20HUD%20Object%20Reference))
  (bind _output_get (Variables|Default|SetCurrentHealth (Variables|Default|GetMaxHealth)))
  (Default|SetHealthBarPercent PlayerHUD _output_get (Variables|Default|GetMaxHealth)))