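; Player attack component for BP_PlayerCharacter_FixedVivian that runs a four-hit melee combo of jab, straight and two hooks.
; IA_Attack plays the montage for the current ComboCount, whose notify unlocks input and advances the count, while a one-second timer resets it.
; StartAttackTrace and StopAttackTrace control a timer-driven, debug-drawn sphere trace from the left or right hand, chosen by ComboCount, that applies damage on hit.
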(event Custom|ResetCount
  (Variables|Default|SetComboCount 0))

(event Custom|AttackTrace
  (bind _playercharacter (Variables|Default|GetPlayerCharacter))
  (bind _playercharacter_2 (Variables|Default|GetPlayerCharacter))
  (bind _righthand (Variables|/Game/NEW/Player/BP_PlayerCharacter_FixedVivian.BP_PlayerCharacter_FixedVivian_C|GetRightHand _playercharacter_2))
  (bind _lefthand (Variables|/Game/NEW/Player/BP_PlayerCharacter_FixedVivian.BP_PlayerCharacter_FixedVivian_C|GetLeftHand _playercharacter))
  (bind (_start _end) (CallFunction|GetHandLocation _lefthand))
  (bind (_start_2 _end_2) (CallFunction|GetHandLocation _righthand))
  (switch int (Variables|Default|GetComboCount)
    (:0
      (bind (_outhit _returnvalue) (Collision|SphereTraceByChannel _start _end 1e+01 "TraceTypeQuery1" false 0 "ForDuration" true "(R=1.000000,G=0.000000,B=0.000000,A=1.000000)" "(R=0.000000,G=1.000000,B=0.000000,A=1.000000)" 7.0 :!label _label))
      (if _returnvalue
        (Game|Damage|ApplyDamage (.HitActor (Collision|BreakHitResult _outhit)) 1e+01 0 (Variables|Default|GetPlayerCharacter))))
    (:1
      (bind (_outhit_2 _returnvalue_2) (Collision|SphereTraceByChannel _start_2 _end_2 1e+01 "TraceTypeQuery1" false 0 "ForDuration" true "(R=1.000000,G=0.000000,B=0.000000,A=1.000000)" "(R=0.000000,G=1.000000,B=0.000000,A=1.000000)" 7.0 :!label _label_2))
      (if _returnvalue_2
        (Game|Damage|ApplyDamage (.HitActor (Collision|BreakHitResult _outhit_2)) 1e+01 0 (Variables|Default|GetPlayerCharacter))))
    (:2
      (goto _label))
    (:3
      (goto _label_2))))

(event Custom|StartAttackTrace
  (bind _returnvalue (Utilities|Time|SetTimerbyEvent (delegate Custom|AttackTrace) 0.01))
  (Variables|Default|SetAttackTimerHandler _returnvalue))

(event Custom|StopAttackTrace
  (Utilities|Time|ClearandInvalidateTimerbyHandle (Variables|Default|GetAttackTimerHandler)))

(event Input|EnhancedActionEvents|EnhancedInputActionIA_Attack
  (params (ActionValue :type Boolean) (ElapsedSeconds :type Float%20%28double-precision%29) (TriggeredSeconds :type Float%20%28double-precision%29) (InputAction :type Input%20Action%20Object%20Reference :default "/Game/NEW/Player/Inputs/IA_Attack.IA_Attack"))
  (bind _charactermesh (Variables|Default|GetCharacterMesh))
  (bind _charactermesh_2 (Variables|Default|GetCharacterMesh))
  (:Started
    (if (not (Variables|Default|GetIsAttacking)) ; 공격 중이 아닐때 만 TRUE
      (Variables|Default|SetIsAttacking true)
      (switch int (Variables|Default|GetComboCount) ; Swith case문
        (:0
          (Animation|Montage|PlayMontage _charactermesh_2 "/Game/NEW/Animations/Montages/Attack1_Jab_Montage.Attack1_Jab_Montage" ; 캐릭터의 애니메이션 조절
            (:then
              (Utilities|Time|SetTimerbyEvent (delegate Custom|ResetCount) 1.0 :!label _label))
            (:OnNotifyBegin
              (Variables|Default|SetIsAttacking false)
              (Variables|Default|SetComboCount 1))))
        (:1
          (Animation|Montage|PlayMontage _charactermesh_2 "/Game/NEW/Animations/Montages/Attack2_Straight_Montage.Attack2_Straight_Montage"
            (:then
              (goto _label))
            (:OnNotifyBegin
              (Variables|Default|SetIsAttacking false)
              (Variables|Default|SetComboCount 2))))
        (:2
          (Animation|Montage|PlayMontage _charactermesh "/Game/NEW/Animations/Montages/Attack3_Hook_Montage.Attack3_Hook_Montage"
            (:then
              (goto _label))
            (:OnNotifyBegin
              (Variables|Default|SetIsAttacking false)
              (Variables|Default|SetComboCount 3))))
        (:3
          (Animation|Montage|PlayMontage _charactermesh "/Game/NEW/Animations/Montages/Attack4_Hook_Montage.Attack4_Hook_Montage"
            (:then
              (goto _label))
            (:OnNotifyBegin
              (Variables|Default|SetIsAttacking false)
              (Variables|Default|SetComboCount 0))))))))

(event EventBeginPlay
  (bind _asbp_player_character_fixed_vivian (Utilities|Casting|CastToBP_PlayerCharacter_FixedVivian (Components|GetOwner)))
  (bind _output_get (Variables|Default|SetPlayerCharacter _asbp_player_character_fixed_vivian))
  (Variables|Default|SetCharacterMesh (Variables|/Script/Engine.Character|GetMesh _output_get)))

(fn GetHandLocation
  (params (Hand :type Scene%20Component%20Object%20Reference))
  (return (Transformation|GetWorldLocation Hand) (Math|Transform|TransformLocation (Transformation|GetWorldTransform Hand) (+ (Variables|/Script/Engine.SceneComponent|GetRelativeLocation Hand) (Math|Vector|MakeVector 2e+01 0.0 0.0)))) ; 퓨어 함수로 변경 > 함수의 입력출력 단계를 안만듦.
)