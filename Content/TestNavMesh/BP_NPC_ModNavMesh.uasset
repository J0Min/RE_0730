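; BP_NPC_ModNavMesh is an NPC that wanders between targets on the navmesh, under the TestNavMesh folder.
; From BeginPlay, MoveNPC picks a random TargetList entry and uses AIMoveTo toward a random reachable point near it.
; It calls itself again after a pause on success or a brief delay on failure, but stops looping if the target is invalid.
; Tick prints the current target and destination for debugging.
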(event Custom|MoveNPC
  (bind _targetlist (Variables|Default|GetTargetList))
  (bind _output_get (Variables|Default|SetCurrentTarget (Utilities|Array|Get(acopy) _targetlist (Math|Random|RandomIntegerinRange 0 (Utilities|Array|LastIndex _targetlist)))))
  (Utilities|IsValid _output_get
    (:Is%20Valid
      (bind _output_get_2 (Variables|Default|SetRandom%20Location (.RandomLocation (AI|Navigation|GetRandomReachablePointinRadius (Transformation|GetActorLocation (Variables|Default|GetCurrentTarget)) 1e+02 0 0))))
      (AI|AIMoveTo self _output_get_2 0 5.0 false
        (:OnSuccess
          (Utilities|FlowControl|Delay 4.0)
          (CallFunction|MoveNPC))
        (:OnFail
          (Utilities|FlowControl|Delay 0.1)
          (CallFunction|MoveNPC))))))

(event EventBeginPlay
  (CallFunction|MoveNPC))

(event EventTick
  (params (DeltaSeconds :type Float%20%28single-precision%29))
  (Development|PrintString (Utilities|GetDisplayName (Variables|Default|GetCurrentTarget)) true true "(R=0.000000,G=0.660000,B=1.000000,A=1.000000)" 2.0 "1")
  (Development|PrintString (Utilities|String|ToString(Vector) (Variables|Default|GetRandom%20Location)) true true "(R=0.000000,G=0.660000,B=1.000000,A=1.000000)" 2.0 "21"))

(fn ConstructionScript)